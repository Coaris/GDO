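; BP_GameTile is a pooled track tile that is recycled as the player passes it.
; When the player overlaps Coll_Used, it messages the player to speed up, then asks TileManager to take out a new tile and put this one back.
; StartUsing has test logic that requests a coin from the PoolManager found at BeginPlay, parented to the tile.
; EndUsing returns the tile's pickups to their pool.
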(event OnComponentBeginOverlap(Coll_Used)
  (params (OverlappedComponent :type Primitive%20Component%20Object%20Reference) (OtherActor :type Actor%20Object%20Reference) (OtherComp :type Primitive%20Component%20Object%20Reference) (OtherBodyIndex :type Integer) (bFromSweep :type Boolean) (SweepResult :type Hit%20Result%20Structure%20%28by%20ref%29))
  (bind _tilemanager (Variables|Default|GetTileManager))
  ;[1 1 1] Set a new game tile from tile manager
  (bind _asbp_player (Utilities|Casting|CastToBP_Player OtherActor))
  (Class|BPIPlayer|SpeedUp(Message) _asbp_player)
  (Class|BPITileManager|ApplyforTakeOutTile(Message) _tilemanager false)
  (Class|BPITileManager|ApplyforPutBackTile(Message) _tilemanager self))

(event EventBeginPlay
  (|CallParentFunction)
  ;[1 1 1] Get reference of pool manager
  (bind _returnvalue (Actor|GetActorOfClass "/Game/Jiale/BP/ReusableActor/BP_PoolManager.BP_PoolManager_C"))
  (Variables|Default|SetPoolManager _returnvalue))

(event EventStartUsing
  (params (TargetLocation :type Vector :default "0, 0, 0"))
  ;[1 0.01979 0.01979] Test
  (|CallParentFunction TargetLocation)
  (Class|BPIPoolManager|ApplyforTakeOut(Message) (Variables|Default|GetPoolManager) "/Game/Jiale/BP/ReusableActor/Collection/BP_RA_Coin.BP_RA_Coin_C" "1000.000000,0.000000,100.000000" self))

(event EventEndUsing
  ;[1 1 1] Let pickups on this tile to return back their pool, when this tile is passed by player
  (|CallParentFunction)
  (Default|CallReturntoPool))

(fn ConstructionScript
  (|CallParentFunction))