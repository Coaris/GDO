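; BP_TileMaster is a tile actor that is reused by toggling between an active and a parked state.
; On BeginPlay it stores its placed location, caches BP_TileManager and the BP_GIBP game instance, then parks itself.
; StartUsing moves it to a target, shows it with NextLocation kept hidden, and enables query-only collision on CollUsed.
; EndUsing returns it to the stored location, hides it and disables that collision, pooling-style.
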(event Custom|StartUsing
  (params (TargetLocation :type Vector))
  ;[1 1 1] Go to target location and be visible
  (Transformation|SetActorLocation TargetLocation false false)
  (Development|SetHiddeninGame (Variables|Default|GetRoot) false true)
  (Development|SetHiddeninGame (Variables|Default|GetNextLocation) true true)
  (Collision|SetCollisionEnabled (Variables|Default|GetColl_Used) "QueryOnly"))

(event Custom|EndUsing
  ;[1 1 1] Go back to start location and be unvisible
  (Transformation|SetActorLocation (Variables|Default|GetUnusingLocation) false false)
  (Development|SetHiddeninGame (Variables|Default|GetRoot) true true)
  (Collision|SetCollisionEnabled (Variables|Default|GetColl_Used) "NoCollision"))

(event EventBeginPlay
  ;[1 1 1] Store start location
  (Variables|Default|SetUnusingLocation (Transformation|GetActorLocation))
  ;[1 1 1] Get reference of tile manager
  (bind _returnvalue (Actor|GetActorOfClass "/Game/Jiale/BP/Tile/BP_TileManager.BP_TileManager_C"))
  (Variables|Default|SetTileManager _returnvalue)
  ;[1 1 1] Get GIBP reference
  (bind _asbp_gibp (Utilities|Casting|CastToBP_GIBP (Game|GetGameInstance)))
  (Variables|Default|SetGameInstance _asbp_gibp)
  ;[1 1 1] Initialize
  (CallFunction|EndUsing))

(fn ConstructionScript)