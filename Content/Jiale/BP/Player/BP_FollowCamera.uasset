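; BP_FollowCamera is a camera actor that follows the player at a fixed height.
; On BeginPlay it becomes player controller 0's view target, caches the BP_Player pawn and records a height from the player's capsule plus a Z offset.
; Each Tick it moves its Sphere component to the capsule's X plus an offset and its Y, holding that initial height so the player's vertical movement is ignored.
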(event EventBeginPlay
  ;[1 1 1] Set Camera
  (Game|Player|SetViewTargetwithBlend (Game|GetPlayerController 0) self 0.0 "VTBlend_Linear" 0.0 false)
  ;[1 1 1] Get Player reference
  (bind _asbp_player (Utilities|Casting|CastToBP_Player (Game|Player|GetPlayerPawn 0)))
  (bind _output_get (Variables|Default|SetPlayer _asbp_player))
  ;[1 1 1] Set Initial location
  (Transformation|SetWorldLocation (Variables|Default|GetSphere) (Math|Vector|MakeVector (+ (.x (Transformation|GetWorldLocation (Variables|/Script/Engine.Character|GetCapsuleComponent _output_get))) (Variables|Default|GetOffsetX)) (.y (Transformation|GetWorldLocation (Variables|/Script/Engine.Character|GetCapsuleComponent _output_get))) (+ (.z (Transformation|GetWorldLocation (Variables|/Script/Engine.Character|GetCapsuleComponent _output_get))) (Variables|Default|GetOffsetZ))) false false)
  (Variables|Default|SetCameraHight (+ (.z (Transformation|GetWorldLocation (Variables|/Script/Engine.Character|GetCapsuleComponent _output_get))) (Variables|Default|GetOffsetZ))))

(event EventTick
  (params (DeltaSeconds :type Float%20%28single-precision%29))
  (bind _player (Variables|Default|GetPlayer))
  (bind _capsulecomponent (Variables|/Script/Engine.Character|GetCapsuleComponent _player))
  (bind _returnvalue (Transformation|GetWorldLocation _capsulecomponent))
  ;[1 1 1] 定高跟随
  (Transformation|SetWorldLocation (Variables|Default|GetSphere) (Math|Vector|MakeVector (+ (.x _returnvalue) (Variables|Default|GetOffsetX)) (.y _returnvalue) (Variables|Default|GetCameraHight)) false false))

(fn ConstructionScript)