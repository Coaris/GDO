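; BP_GameMode is the game mode that prepares the tile-based level before play starts.
; On BeginPlay it finds the BP_TileManager in the world and caches the BP_GIBP game instance.
; It then asks the tile manager to take out tiles once per StartTileAmount to set up the starting tiles.
; A disconnected debug branch that would flag the game as started after a delay never runs.
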(event EventBeginPlay
  (Utilities|FlowControl|Sequence
    (:then_0
      ;[1 1 1] Get tile manager reference
      (bind _returnvalue (Actor|GetActorOfClass "/Game/Jiale/BP/Tile/BP_TileManager.BP_TileManager_C"))
      (Variables|References|SetTileManager _returnvalue)
      ;[1 1 1] Get game instance reference
      (bind _asbp_gibp (Utilities|Casting|CastToBP_GIBP (Game|GetGameInstance)))
      (Variables|References|SetGameInstance _asbp_gibp)
      ;[1 1 1] Setup start tiles for preparing game start
      (for _index (range 1 (Variables|Setup|GetStartTileAmount))
        (Class|BPITileManager|ApplyforTakeOutTile(Message) (Variables|References|GetTileManager) true)))))

(fn ConstructionScript)