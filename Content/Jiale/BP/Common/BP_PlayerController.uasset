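; BP_PlayerController is a player controller that toggles the game's pause state and PC pause menu.
; The IA_Pause input and the PauseOrResume event share one toggle driven by IsPaused.
; Pausing creates a fresh WBP_PauseMenu_PC, focuses it and pauses the game.
; Resuming removes that widget, unpauses and returns focus to GamePlayPC, keeping Game and UI input mode.
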(event Custom|PauseOrResume
  (bind _returnvalue (Game|GetPlayerController 0))
  (if (Variables|Default|GetIsPaused)
    ;[1 1 1] Resume
    (Variables|Default|SetIsPaused false)
    (Widget|RemovefromParent (Variables|Default|GetPauseMenuPC))
    (Game|SetGamePaused false)
    (Input|SetInputModeGameandUI _returnvalue (Variables|Default|GetGamePlayPC) "DoNotLock" false false)
    (else
      ;[1 1 1] Pause
      (Variables|Default|SetIsPaused true)
      (bind _returnvalue_2 (UserInterface|CreateWidget "/Game/Jiale/UI/WBP_PauseMenu_PC.WBP_PauseMenu_PC_C" _returnvalue))
      (bind _output_get (Variables|Default|SetPauseMenuPC _returnvalue_2))
      (UserInterface|Viewport|AddtoViewport _output_get 0)
      (Input|SetInputModeGameandUI _returnvalue (Variables|Default|GetPauseMenuPC) "DoNotLock" false false)
      (Game|SetGamePaused true))))

(event Input|EnhancedActionEvents|EnhancedInputActionIA_Pause
  (params (ActionValue :type Boolean) (ElapsedSeconds :type Float%20%28double-precision%29) (TriggeredSeconds :type Float%20%28double-precision%29) (InputAction :type Input%20Action%20Object%20Reference :default "/Game/Jiale/Input/IA_Pause.IA_Pause"))
  (bind _returnvalue (Game|GetPlayerController 0))
  (:Started
    (if (Variables|Default|GetIsPaused)
      ;[1 1 1] Resume
      (Variables|Default|SetIsPaused false)
      (Widget|RemovefromParent (Variables|Default|GetPauseMenuPC))
      (Game|SetGamePaused false)
      (Input|SetInputModeGameandUI _returnvalue (Variables|Default|GetGamePlayPC) "DoNotLock" false false)
      (else
        ;[1 1 1] Pause
        (Variables|Default|SetIsPaused true)
        (bind _returnvalue_2 (UserInterface|CreateWidget "/Game/Jiale/UI/WBP_PauseMenu_PC.WBP_PauseMenu_PC_C" _returnvalue))
        (bind _output_get (Variables|Default|SetPauseMenuPC _returnvalue_2))
        (UserInterface|Viewport|AddtoViewport _output_get 0)
        (Input|SetInputModeGameandUI _returnvalue (Variables|Default|GetPauseMenuPC) "DoNotLock" false false)
        (Game|SetGamePaused true)))))

(event Input|EnhancedActionEvents|EnhancedInputActionIA_Test
  (params (ActionValue :type Boolean) (ElapsedSeconds :type Float%20%28double-precision%29) (TriggeredSeconds :type Float%20%28double-precision%29) (InputAction :type Input%20Action%20Object%20Reference :default "/Game/Jiale/Input/IA_Test.IA_Test"))
  ;[1 0.2789 0.2729] Test
)

(fn ConstructionScript)