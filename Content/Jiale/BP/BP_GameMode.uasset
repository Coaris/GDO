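; Game mode Blueprint that prepares the start tiles and flags the game as started on BeginPlay.
; It finds BP_TileManager and the BP_GIBP game instance, then requests a take-out tile from the manager once per StartTileAmount.
; A second sequence step, marked as debug, immediately sets IsGameStart on the game instance, leaving a five-second delay node unused.
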(event EventBeginPlay
  (Utilities|FlowControl|Sequence
    (:then_0
      ;[1 1 1] Get tile manager reference
      (bind _returnvalue (Actor|GetActorOfClass "/Game/Jiale/BP/Tile/BP_TileManager.BP_TileManager_C"))
      (Variables|References|SetTileManager _returnvalue)
      ;[1 1 1] Get game instance reference
      (bind _asbp_gibp (Utilities|Casting|CastToBP_GIBP (Game|GetGameInstance)))
      (Variables|References|SetGameInstance _asbp_gibp)
      ;[1 1 1] Setup start tiles for preparing game start
      (for _index (range 1 (Variables|Setup|GetStartTileAmount))
        (Class|BPITileManager|ApplyforTakeOutTile(Message) (Variables|References|GetTileManager) true)))
    (:then_1
      ;[1 0.1448 0.1448] Debug
      (Variables|/Game/Jiale/BP/BP_GIBP.BP_GIBP_C|SetIsGameStart (Variables|References|GetGameInstance) true))))

(fn ConstructionScript)