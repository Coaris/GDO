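; BP_GIBP, apparently the Game Instance, manages the game's start and end and keeps the farthest distance and total coins.
; StartGame raises the start flag and event, messages BP_Player and binds EndGame to the GameOver event.
; EndGame shows the game-over widget with UI-only input, pauses, and saves.
; SaveGame loads or creates BP_SaveGame in the "Score" slot, then writes both totals to it.
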(event Custom|StartGame
  ;[1 1 1] Game start & End
  (Variables|Default|SetIsGameStart true)
  (Default|CallGameStart)
  (bind _asbp_player (Utilities|Casting|CastToBP_Player (Game|Player|GetPlayerPawn 0)))
  (bind _output_get (Variables|Default|SetPlayer _asbp_player))
  (Class|BPIPlayer|Start(Message) _output_get)
  (EventDispatchers|BindEventtoGameOver (delegate Custom|EndGame)))

(event Custom|EndGame
  (bind _returnvalue (Game|GetPlayerController 0))
  ;[1 1 1] Game start & End
  (Variables|Default|SetIsGameStart false)
  (bind _returnvalue_2 (UserInterface|CreateWidget "/Game/Jiale/UI/WBP_GameOver_PC.WBP_GameOver_PC_C" _returnvalue))
  (UserInterface|Viewport|AddtoViewport _returnvalue_2 0)
  (Input|SetInputModeUIOnly _returnvalue _returnvalue_2 "DoNotLock" false)
  (Game|SetGamePaused true)
  (CallFunction|SaveGame))

(fn RecordBestScore
  (params (DIstance :type Integer))
  (if (> DIstance (Variables|Default|GetFarthestDistance))
    (Variables|Default|SetFarthestDistance (Variables|Default|GetDistance))))

(fn CalcTotalCoin
  (params (Coin :type Integer))
  (Variables|Default|SetTotalCoin (+ Coin (Variables|Default|GetTotalCoin))))

(fn SaveGame
  (bind _returnvalue (SaveGame|DoesSaveGameExist "Score"))
  (if _returnvalue
    ;[1 1 1] There is a SaveGame
    (bind _returnvalue_2 (SaveGame|LoadGamefromSlot "Score"))
    (bind _asbp_save_game (Utilities|Casting|CastToBP_SaveGame _returnvalue_2))
    (Variables|Default|SetSaveGameData _asbp_save_game)
    (else
      ;[1 1 1] There is no Save Game
      (bind _returnvalue_3 (SaveGame|CreateSaveGameObject "/Game/Jiale/BP/SaveGame/BP_SaveGame.BP_SaveGame_C"))
      (Variables|Default|SetSaveGameData _returnvalue_3)))
  (Variables|/Game/Jiale/BP/SaveGame/BP_SaveGame.BP_SaveGame_C|SetBestDistance (Variables|Default|GetSaveGameData) (Variables|Default|GetFarthestDistance))
  (Variables|/Game/Jiale/BP/SaveGame/BP_SaveGame.BP_SaveGame_C|SetTotalCoin (Variables|Default|GetSaveGameData) (Variables|Default|GetTotalCoin))
  (bind _returnvalue_4 (SaveGame|SaveGametoSlot (Variables|Default|GetSaveGameData) "Score"))
  (if _returnvalue_4
    (Development|PrintString "Saved")
    (else
      (Development|PrintString "Save Fail"))))