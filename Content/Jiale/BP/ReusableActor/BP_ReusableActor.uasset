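; Base pooled actor that can be shown at a target location and returned to a hidden, collisionless state.
; Initialize stores the owning pool and deactivates the actor; EndUsing moves it back to the location saved at BeginPlay.
; StartUsing unhides it with query-only collision.
; Tick runs the empty Behaviour event while IsUsing is true, but both StartUsing and EndUsing set that flag false.
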(event Custom|StartUsing
  (params (TargetLocation :type Vector))
  ;[1 1 1] Start using
  (Transformation|SetActorRelativeLocation TargetLocation)
  (Transformation|SetActorRelativeRotation "0, 0, 0")
  (Development|SetHiddeninGame (Variables|Default|GetRoot) false true)
  (Collision|SetCollisionEnabled (Variables|Default|GetStaticMesh) "QueryOnly")
  (Variables|Default|SetIsUsing false))

(event Custom|EndUsing
  ;[1 1 1] End using
  (Transformation|SetActorLocationAndRotation (Variables|Default|GetUsingLocation) "0, 0, 0")
  (Development|SetHiddeninGame (Variables|Default|GetRoot) true true)
  (Collision|SetCollisionEnabled (Variables|Default|GetStaticMesh) "NoCollision")
  (Variables|Default|SetIsUsing false))

(event Custom|Initialize
  (params (Pool :type BPAC%20Object%20Pool%20Object%20Reference))
  ;[1 1 1] Get ference of pool
  (Variables|Default|SetPool Pool)
  ;[1 1 1] Hide and Deactive
  (CallFunction|EndUsing))

(event Custom|Behaviour)

(event EventBeginPlay
  ;[1 1 1] Store start location
  (Variables|Default|SetUsingLocation (Transformation|GetActorLocation)))

(event EventTick
  (params (DeltaSeconds :type Float%20%28single-precision%29))
  ;[1 1 1] Active behaviour when actor is actived
  (if (Variables|Default|GetIsUsing)
    (CallFunction|Behaviour)))

(fn ConstructionScript)