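; BP_PoolManager is a central registry that routes object-pooling requests to per-class actor pools.
; Pools are added to PoolList through an event, and GetPool searches that list linearly for an exact ActorClass match.
; Take-out requests pass a target location and parent to the matching pool, while put-back requests find the pool from the returned actor's class.
; GetPool has no explicit fallback for a class without a registered pool.
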(event Custom|AddPoolToPoolList
  (params (Pool :type BPAC%20Object%20Pool%20Object%20Reference))
  ;[1 1 1] Add pool into pool list
  (Utilities|Array|Add (Variables|Default|GetPoolList) Pool))

(event EventApplyforPutBack
  (params (Actor :type BP%20Reusable%20Actor%20Object%20Reference))
  ;[1 1 1] Put actor back to pool
  (bind _pool (CallFunction|GetPool (Utilities|GetClass Actor)))
  (Default|PutBack _pool Actor))

(event EventApplyforTakeOut
  (params (ActorClass :type BP%20Reusable%20Actor%20Class%20Reference) (TargetLocation :type Vector :default "0, 0, 0") (Parent :type Actor%20Object%20Reference))
  ;[1 1 1] Take out an actor by actor class
  (bind _pool (CallFunction|GetPool ActorClass))
  (Default|TakeOut _pool TargetLocation Parent))

(fn ConstructionScript)

(fn GetPool
  (params (ActorClass :type BP%20Reusable%20Actor%20Class%20Reference))
  (bind _array_element (Utilities|Array|ForEachLoopwithBreak (Variables|Default|GetPoolList) :!label _label)
    (:LoopBody
      (if (== (Variables|/Game/Jiale/BP/ReusableActor/BPAC_ObjectPool.BPAC_ObjectPool_C|GetActorClass _array_element) ActorClass)
        (goto _label Break)))
    (:Completed
      (return _array_element))))