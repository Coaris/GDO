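; BP_RA_Collection is a pooled pickup placed on game tiles that spins while in use.
; On StartUsing it registers with its attached parent BP_GameTile's return-to-pool callback, so it goes back to the PoolManager with the tile.
; Overlap by BP_Player calls PickedUp, an empty hook here, then applies to the pool manager to be put back.
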(event OnComponentBeginOverlap(Box)
  (params (OverlappedComponent :type Primitive%20Component%20Object%20Reference) (OtherActor :type Actor%20Object%20Reference) (OtherComp :type Primitive%20Component%20Object%20Reference) (OtherBodyIndex :type Integer) (bFromSweep :type Boolean) (SweepResult :type Hit%20Result%20Structure%20%28by%20ref%29))
  ;[1 1 1] Call PickedUP when player get this collection
  (Utilities|Casting|CastToBP_Player OtherActor)
  (CallFunction|PickedUp)
  (Default|ApplyforPutBack (Variables|Default|GetPoolManager) self))

(event Custom|ReturnToPool_Event
  ;[1 1 1] Be put back pool, when parent tile is passed by player
  (Default|ApplyforPutBack (Variables|Default|GetPoolManager) self))

(event Custom|PickedUp
  ;[1 1 1] Call PickedUP when player get this collection
)

(event EventBeginPlay
  (|CallParentFunction))

(event EventTick
  (params (DeltaSeconds :type Float%20%28single-precision%29))
  ;[1 1 1] Self Rotation
  (if (Variables|Default|GetIsUsing)
    (Transformation|AddLocalRotation (Variables|Default|GetRoot) "0.000000,-2.000000,0.000000" false false)))

(event EventStartUsing
  (params (TargetLocation :type Vector :default "0, 0, 0"))
  ;[1 1 1] Be put back pool, when parent tile is passed by player
  (|CallParentFunction TargetLocation)
  ;;[1 1 1] Get Parent Tile
  (bind _asbp_game_tile (Utilities|Casting|CastToBP_GameTile (Actor|GetAttachParentActor)))
  (EventDispatchers|AssignReturntoPool _asbp_game_tile (delegate Custom|ReturnToPool_Event)))

(fn ConstructionScript
  (|CallParentFunction))