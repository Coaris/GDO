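; BP_RA_Obstacle is a pooled obstacle placed on game tiles that blocks the player.
; On StartUsing, it casts its attach parent to BP_GameTile and binds a return event, so PoolManager reclaims it when the player passes that tile.
; A box overlap with BP_Player calls the empty BlockedDown event and prints "GameOver", with no further game-over logic here.
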(event OnComponentBeginOverlap(Box)
  (params (OverlappedComponent :type Primitive%20Component%20Object%20Reference) (OtherActor :type Actor%20Object%20Reference) (OtherComp :type Primitive%20Component%20Object%20Reference) (OtherBodyIndex :type Integer) (bFromSweep :type Boolean) (SweepResult :type Hit%20Result%20Structure%20%28by%20ref%29))
  ;[1 1 1] Game over, when player blocked by this obstacle
  (Utilities|Casting|CastToBP_Player OtherActor)
  (CallFunction|BlockedDown)
  (Development|PrintString "GameOver"))

(event Custom|BlockedDown
  ;[1 1 1] Game over, when player blocked by this obstacle
)

(event Custom|ReturnToPool_Event
  ;[1 1 1] Be put back pool, when parent tile is passed by player
  (Default|ApplyforPutBack (Variables|Default|GetPoolManager) self))

(event EventBeginPlay
  (|CallParentFunction))

(event EventStartUsing
  (params (TargetLocation :type Vector :default "0, 0, 0"))
  ;[1 1 1] Be put back pool, when parent tile is passed by player
  (|CallParentFunction TargetLocation)
  ;;[1 1 1] Get Parent Tile
  (bind _asbp_game_tile (Utilities|Casting|CastToBP_GameTile (Actor|GetAttachParentActor)))
  (EventDispatchers|AssignReturntoPool _asbp_game_tile (delegate Custom|ReturnToPool_Event)))

(fn ConstructionScript
  (|CallParentFunction))