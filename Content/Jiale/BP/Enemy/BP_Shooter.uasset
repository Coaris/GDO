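; BP_Shooter is an enemy that periodically moves in, signals shots, moves back, and damages the player with a bomb projectile.
; Once BP_GIBP signals game start, a looping timer drives timeline movement of the skeletal mesh and a delayed attack sequence that raises IsShooting.
; Shoot, not called within this graph, clears that flag, lerps the bomb along its path and re-arms the sphere's Pawn overlap, which disables itself after hitting BP_Player.
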(event OnComponentBeginOverlap(Sphere)
  (params (OverlappedComponent :type Primitive%20Component%20Object%20Reference) (OtherActor :type Actor%20Object%20Reference) (OtherComp :type Primitive%20Component%20Object%20Reference) (OtherBodyIndex :type Integer) (bFromSweep :type Boolean) (SweepResult :type Hit%20Result%20Structure%20%28by%20ref%29))
  ;[1 1 1] make damage on player
  (bind _asbp_player (Utilities|Casting|CastToBP_Player OtherActor))
  (Collision|SetCollisionResponsetoChannel (Variables|Default|GetSphere) "ECC_Pawn" "ECR_Ignore")
  (Class|BPIPlayer|GetDamage(Message) _asbp_player))

(event Custom|GameStart_Event
  (Utilities|Time|SetTimerbyEvent (delegate Custom|MoveForward) 3e+01 true))

(event Custom|MoveForward
  ;[1 1 1] Move forward
  (bind _movealpha (Timeline|Timeline PlayFromStart)
    (:Update
      (Transformation|SetRelativeLocation (Variables|Default|GetSkeletalMesh) (Math|Vector|MakeVector (Math|Float|Lerp (Variables|Default|GetStartLocation) (Variables|Default|GetEndLocation) _movealpha) 0.0 2e+02) false false))
    (:Finished
      (CallFunction|Attack))))

(event Custom|MoveBackward
  ;[1 1 1] movw back
  (bind _movealpha (Timeline|Timeline_0 PlayFromStart)
    (:Update
      (Transformation|SetRelativeLocation (Variables|Default|GetSkeletalMesh) (Math|Vector|MakeVector (Math|Float|Lerp (Variables|Default|GetStartLocation) (Variables|Default|GetEndLocation) _movealpha) 0.0 2e+02) false false))))

(event Custom|Attack
  ;[1 1 1] Attack
  (Utilities|FlowControl|Delay 5.0)
  (Variables|Animation|SetIsShooting true)
  (Utilities|FlowControl|Delay 5.0)
  (Variables|Animation|SetIsShooting true)
  (Utilities|FlowControl|Delay 5.0)
  (CallFunction|MoveBackward))

(event EventBeginPlay
  ;[1 1 1] get reference of player
  (bind _asbp_player (Utilities|Casting|CastToBP_Player (Game|Player|GetPlayerPawn 0)))
  (Variables|Reference|SetPlayer _asbp_player)
  (bind _asbp_gibp (Utilities|Casting|CastToBP_GIBP (Game|GetGameInstance)))
  (EventDispatchers|AssignGameStart _asbp_gibp (delegate Custom|GameStart_Event)))

(event EventShoot
  ;[1 1 1] Shoot a bullet
  (Variables|Animation|SetIsShooting false)
  (Collision|SetCollisionResponsetoChannel (Variables|Default|GetSphere) "ECC_Pawn" "ECR_Overlap")
  (bind _lerpalpha (Timeline|BombTimeline PlayFromStart)
    (:Update
      (Transformation|SetRelativeLocation (Variables|Default|GetBomb) (Math|Vector|Lerp(Vector) (Variables|Default|GetBombStartLocation) (Variables|Default|GetBombEndLocation) _lerpalpha) false false))))

(fn ConstructionScript)